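; Runite armor pickup for a 2D side-scroller that floats in place until the player collects it into the inventory.
; Each tick, a rising and falling counter is squared and scaled by Speed to offset the sprite's height from its starting Z.
; Collision overlap flags the player's presence, and Tick polls the character's action input.
; A successful data-table-backed inventory add destroys the actor.
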(event OnComponentBeginOverlap(Collision)
  (params (OverlappedComponent :type Primitive%20Component%20Object%20Reference) (OtherActor :type Actor%20Object%20Reference) (OtherComp :type Primitive%20Component%20Object%20Reference) (OtherBodyIndex :type Integer) (bFromSweep :type Boolean) (SweepResult :type Hit%20Result%20Structure%20%28by%20ref%29))
  (Utilities|Casting|CastTo2DSideScrollerCharacter OtherActor)
  (Variables|Default|SetPlayerOverlap true))

(event OnComponentEndOverlap(Collision)
  (params (OverlappedComponent :type Primitive%20Component%20Object%20Reference) (OtherActor :type Actor%20Object%20Reference) (OtherComp :type Primitive%20Component%20Object%20Reference) (OtherBodyIndex :type Integer))
  (Utilities|Casting|CastTo2DSideScrollerCharacter OtherActor)
  (Variables|Default|SetPlayerOverlap false))

(event Custom|FloatAnim
  (bind _sprite (Variables|Default|GetSprite))
  (bind _returnvalue (Transformation|GetWorldLocation _sprite))
  ;[1 1 1] Floating Animation
  (if (Variables|Default|GetHeightRising)
    (if (>= (Variables|Default|GetCurrentFloatingHeight) 1e+02)
      (Variables|Default|SetHeightRising false :!label _label)
      (Variables|Default|SetCurrentFloatingHeight (- (Variables|Default|GetCurrentFloatingHeight) 1.0))
      (else
        (Variables|Default|SetHeightRising true :!label _label_2)
        (Variables|Default|SetCurrentFloatingHeight (+ (Variables|Default|GetCurrentFloatingHeight) 1.0))))
    (elif (<= (Variables|Default|GetCurrentFloatingHeight) 0.0)
      (if (== (Variables|Default|GetRevolution) 1)
        (Variables|Default|SetRevolution 2)
        (goto _label_2)
        (else
          (Variables|Default|SetRevolution 1)
          (CallFunction|SwitchFloating)
          (goto _label_2)))
      (else
        (goto _label))))
  (bind _output_get (Variables|Default|SetFloatingLocation (+ (Variables|Default|GetStartingLocation) (* (* (Variables|Default|GetCurrentFloatingHeight) (Variables|Default|GetCurrentFloatingHeight)) (Variables|Default|GetSpeed)))))
  (Transformation|SetWorldLocation (Variables|Default|GetSprite) (Math|Vector|MakeVector (.x _returnvalue) (.y _returnvalue) _output_get) false false))

(event Custom|SwitchFloating
  ;[1 1 1] Floating Animation
  (if (Variables|Default|GetFloatingUp)
    (Variables|Default|SetFloatingUp false)
    (else
      (Variables|Default|SetFloatingUp true))))

(event EventBeginPlay
  ;[1 1 1] Floating Animation
  (Variables|Default|SetStartingLocation (.z (Transformation|GetWorldLocation (Variables|Default|GetSprite)))))

(event EventTick
  (params (DeltaSeconds :type Float%20%28single-precision%29))
  (CallFunction|FloatAnim)
  (bind _as2dside_scroller_character (Utilities|Casting|CastTo2DSideScrollerCharacter (Game|GetPlayerCharacter 0)))
  (if (and (Variables|/Game/Character/2DSideScrollerCharacter.2DSideScrollerCharacter_C|GetActionPressed _as2dside_scroller_character) (Variables|Default|GetPlayerOverlap))
    (bind _added (Default|AddNewInventoryItem :self (Variables|/Game/Widgets/Inventory.Inventory_C|GetInventorySlot (Variables|/Game/Character/2DSideScrollerCharacter.2DSideScrollerCharacter_C|GetInventory _as2dside_scroller_character)) :ItemID "RuniteArmor" :Count 1 :InDataTable "/Game/Widgets/Inv_DataTable.Inv_DataTable"))
    (if _added
      (Actor|DestroyActor))))

(fn ConstructionScript)
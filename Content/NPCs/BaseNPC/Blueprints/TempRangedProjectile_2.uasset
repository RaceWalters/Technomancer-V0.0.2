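; NPC ranged projectile for the side-scroller, locked to Y=0 every tick.
; BeginPlay sets lifespan from a Range tier divided by max speed; Tick counts it down per frame, so travel distance depends on frame rate.
; An active player Speculum Hypershield can reflect it, reversing velocity, flipping pitch and making the player Instigator.
; Optional flags destroy it on Holoshields, non-instigator NPCs (after short delays) or blocking hits.
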(event OnComponentHit(CollisionBox)
  (params (HitComponent :type Primitive%20Component%20Object%20Reference) (OtherActor :type Actor%20Object%20Reference) (OtherComp :type Primitive%20Component%20Object%20Reference) (NormalImpulse :type Vector :default "0, 0, 0") (Hit :type Hit%20Result%20Structure%20%28by%20ref%29))
  ;[1 1 1] Destroy on Contact w/ Obstacle
  (if (Variables|Default|GetDestroyedOnTileImpact)
    (Actor|DestroyActor)))

(event OnComponentBeginOverlap(CollisionBox)
  (params (OverlappedComponent :type Primitive%20Component%20Object%20Reference) (OtherActor :type Actor%20Object%20Reference) (OtherComp :type Primitive%20Component%20Object%20Reference) (OtherBodyIndex :type Integer) (bFromSweep :type Boolean) (SweepResult :type Hit%20Result%20Structure%20%28by%20ref%29))
  (bind _collision_box (Variables|Default|GetCollision%20Box))
  (bind _projectilemovement (Variables|Default|GetProjectileMovement))
  (bind _returnvalue (Transformation|GetWorldRotation _collision_box))
  ;[1 1 1] Destroy Self on Holoplate if Check
  ;[1 1 1] Check for Speculum Hypershield if Checked
  (if (and (Variables|Default|GetDeflectedBySpeculumHypershield) (Components|ComponentHasTag OtherComp "Player"))
    (bind _as2dside_scroller_character (Utilities|Casting|CastTo2DSideScrollerCharacter (Game|GetPlayerCharacter 0)))
    (if (Variables|/Game/Character/2DSideScrollerCharacter.2DSideScrollerCharacter_C|GetSpeculumHypershieldActive _as2dside_scroller_character)
      (Variables|/Script/Engine.MovementComponent|SetVelocity _projectilemovement (* (Variables|/Script/Engine.MovementComponent|GetVelocity _projectilemovement) -1))
      (Transformation|SetWorldRotation _collision_box (Math|Rotator|MakeRotator (.roll _returnvalue) (+ (.pitch _returnvalue) 1.8e+02) (.yaw _returnvalue)) false false)
      (Variables|Actor|SetInstigator self _as2dside_scroller_character)
      (else
        (if (and (Components|ComponentHasTag OtherComp "Holoshield") (Variables|Default|GetDestroyedOnHoloshield)) :!label _label
          (Actor|DestroyActor)
          (else
            (Utilities|FlowControl|Delay 0.01)
            (if (Variables|Default|GetDestroyedOnNPCImpact)
              (if (Components|ComponentHasTag OtherComp "NPC")
                (if (not (== OtherActor (Game|GetInstigator)))
                  (Utilities|FlowControl|Delay 0.01)
                  (Actor|DestroyActor))))))))
    (else
      (goto _label))))

(event EventTick
  (params (DeltaSeconds :type Float%20%28single-precision%29))
  (bind _collision_box (Variables|Default|GetCollision%20Box))
  (bind _returnvalue (Transformation|GetWorldLocation _collision_box))
  ;[1 1 1] Keep On 0 Y
  (Transformation|SetWorldLocation _collision_box (Math|Vector|MakeVector (.x _returnvalue) 0.0 (.z _returnvalue)) false false)
  ;[1 1 1] Lifespan Decay
  (Variables|Default|SetLifespanDecay (- (Variables|Default|GetLifespanDecay) 1.0))
  (if (<= (- (Variables|Default|GetLifespanDecay) 1.0) 0.0)
    (Actor|DestroyActor)))

(event EventBeginPlay
  ;[1 1 1] Decide Lifespan Based on Speed
  (if (== (Variables|Default|GetRange) 0)
    (Variables|Default|SetLifespanDecay (* 5000 (/ 1.0 (Class|MovementComponent|GetMaxSpeed (Variables|Default|GetProjectileMovement)))))
    (elif (== (Variables|Default|GetRange) 1)
      (Variables|Default|SetLifespanDecay (* 25000 (/ 1.0 (Class|MovementComponent|GetMaxSpeed (Variables|Default|GetProjectileMovement)))))
      (elif (== (Variables|Default|GetRange) 2)
        (Variables|Default|SetLifespanDecay (* 50000 (/ 1.0 (Class|MovementComponent|GetMaxSpeed (Variables|Default|GetProjectileMovement)))))
        (elif (== (Variables|Default|GetRange) 3)
          (Variables|Default|SetLifespanDecay (* 100000 (/ 1.0 (Class|MovementComponent|GetMaxSpeed (Variables|Default|GetProjectileMovement)))))
          (elif (== (Variables|Default|GetRange) 4)
            (Variables|Default|SetLifespanDecay (* 1000000 (/ 1.0 (Class|MovementComponent|GetMaxSpeed (Variables|Default|GetProjectileMovement)))))))))))

(fn ConstructionScript)